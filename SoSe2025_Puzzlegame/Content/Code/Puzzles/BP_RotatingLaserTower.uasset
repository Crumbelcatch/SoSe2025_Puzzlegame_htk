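; Interactable puzzle laser tower that rotates between evenly spaced sides and powers whatever actor its beam hits.
; The construction script builds the yaw steps from Sides and warns if CorrectSide exceeds them; interacting eases to the next via a timeline.
; While powered and stationary, a Delay-throttled Tick line-traces forward, updating the Niagara beam endpoint.
; Trigger messages switch hit actors on and previous ones off, and also set the tower's own power.
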(event Custom|Rotate
  ;[0 0.6997 0.6456 0.5] Rotate Function
  (bind _alpha (Timeline|SmoothRotate PlayFromStart)
    (:Update
      (Transformation|SetRelativeRotation (Variables|Default|GetMeshPivot) (Math|Rotator|MakeRotator 0.0 0.0 (.yaw (Math|Rotator|Lerp(Rotator) (Math|Rotator|MakeRotator 0.0 0.0 (Variables|Default|GetCurrentRotation)) (Math|Rotator|MakeRotator 0.0 0.0 (Utilities|Array|Get(acopy) (Variables|Default|GetNumbersRotation) (Variables|Default|GetCurrentSide))) _alpha true))) false false))
    (:Finished
      (Variables|Default|SetCurrentRotation (.yaw (Variables|/Script/Engine.SceneComponent|GetRelativeRotation (Variables|Default|GetMeshPivot)))))))

(event Custom|Pew
  (bind _beam (Variables|Default|GetBeam))
  (bind _directionalarrow (Variables|Default|GetDirectionalArrow))
  (bind _returnvalue (Transformation|GetWorldLocation _directionalarrow))
  ;[0 0.5828 1 0.5] Pew
  (if (Variables|Default|GetIsPowerd)
    (bind _outhit (Collision|LineTraceByChannel _returnvalue (+ _returnvalue (* (Math|Vector|GetForwardVector _directionalarrow) (Variables|Default|GetLaserLength))) "TraceTypeQuery1" false 0 "ForDuration" true "(R=1.000000,G=0.000000,B=0.000000,A=1.000000)" "(R=0.000000,G=1.000000,B=0.000000,A=1.000000)" 2.0))
    (if (== (Variables|Default|GetLast%20Hit%20Actor) (.HitActor (Collision|BreakHitResult _outhit)))
      _
      (else
        (Class|BPITrigger|Trigger(Message) (Variables|Default|GetLast%20Hit%20Actor) 0 false)
        (Variables|Default|SetLast%20Hit%20Actor (.HitActor (Collision|BreakHitResult _outhit)))))
    (if (.bBlockingHit (Collision|BreakHitResult _outhit))
      (Components|Activation|SetActive _beam true false)
      (Niagara|SetNiagaraVariable(Vector3) _beam "EndLocation" (.ImpactPoint (Collision|BreakHitResult _outhit)))
      (Class|BPITrigger|Trigger(Message) (.HitActor (Collision|BreakHitResult _outhit)) 0 true)
      (else
        (Components|Activation|SetActive (Variables|Default|GetBeam) false false)))
    (else
      (Components|Activation|SetActive (Variables|Default|GetBeam) false false))))

(event EventTick
  (params (DeltaSeconds :type Float%20%28single-precision%29))
  (Utilities|FlowControl|Delay 0.2)
  (if (not (Audio|Components|Audio|IsPlaying (Variables|Default|GetSmoothRotate)))
    (CallFunction|Pew)))

(event EventSetHighlight
  (params (ShowOverlay :type Boolean))
  (Rendering|Material|SetOverlayMaterial (Variables|Default|GetBLOCKOUT_Octagon) (select ShowOverlay "/Game/BLOCKOUT/MapV1_Mat.MapV1_Mat" 0) :!class /Script/Engine.MeshComponent))

(event EventInteract
  ;[0 0.6997 0.6456 0.5] Interact
  (if (not (Audio|Components|Audio|IsPlaying (Variables|Default|GetSmoothRotate)))
    (Math|Integer|IncrementInt (Variables|Default|GetCurrentSide)
      (:%20%20
        (if (== (Variables|Default|GetCurrentSide) (Utilities|Array|Length (Variables|Default|GetNumbersRotation)))
          (Variables|Default|SetCurrentSide 0))
        (CallFunction|Rotate)))))

(event EventTrigger
  (params (ActorRef :type Actor%20Object%20Reference) (RemoveActorRef :type Boolean))
  (bind _output_get (Variables|Default|SetIsPowerd RemoveActorRef))
  (if _output_get
    (CallFunction|Pew)
    (else
      (Class|BPITrigger|Trigger(Message) (Variables|Default|GetLast%20Hit%20Actor) 0 false)
      (Variables|Default|SetLast%20Hit%20Actor 0))))

(fn ConstructionScript
  (Variables|Default|SetSegmentSize (/ 360 (Variables|Default|GetSides)))
  (for _index (range 0 (Variables|Default|GetSides))
    (if (> 3.6e+02 (* _index (Variables|Default|GetSegmentSize)))
      (Utilities|Array|SetArrayElem (Variables|Default|GetNumbersRotation) _index (* _index (Variables|Default|GetSegmentSize)) true)
      (if (> (Variables|Default|GetCorrectSide) (Variables|Default|GetSides))
        (Development|PrintString (Utilities|String|Append (Utilities|GetDisplayName self) " is unsolvable!  Variable: CorrectSide is bigger than Total Sides") true true "(R=1.000000,G=0.078514,B=0.000000,A=1.000000)" 1e+01)
        (Variables|Default|SetCurrentSide 0)))))

(fn CustomInteractPrompt
  (return ""))

(fn IsInteractable
  (return (Variables|Default|GetIs%20Interactable)))