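; Puzzle actor that slides its mesh toward an EndPoint component's position when triggered.
; Trigger stores the mesh's relative location, then plays the SmoothSlide timeline to lerp it toward EndPoint, feeding in only X and Y.
; The construction script sets the timeline's play rate from AnimationSpeed.
; No reverse movement is defined, and BeginPlay, overlap and Tick are empty.
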(event EventBeginPlay)

(event Collision|EventActorBeginOverlap
  (params (OtherActor :type Actor%20Object%20Reference)))

(event EventTick
  (params (DeltaSeconds :type Float%20%28single-precision%29)))

(event EventTrigger
  (params (ActorRef :type Actor%20Object%20Reference) (RemoveActorRef :type Boolean))
  (bind _endpoint (Variables|Default|GetEndPoint))
  (bind _relativelocation (Variables|/Script/Engine.SceneComponent|GetRelativeLocation _endpoint))
  (Variables|Default|SetRelative%20Location (Variables|/Script/Engine.SceneComponent|GetRelativeLocation (Variables|Default|GetMesh)))
  (bind _alpha (Timeline|SmoothSlide Play)
    (:Update
      (Transformation|SetRelativeLocation (Variables|Default|GetMesh) (Math|Vector|Lerp(Vector) (Math|Vector|MakeVector (.x (Variables|Default|GetRelative%20Location)) (.y (Variables|Default|GetRelative%20Location)) 0.0) (Math|Vector|MakeVector (.x _relativelocation) (.y _relativelocation) 0.0) _alpha) false false))))

(fn ConstructionScript
  (Components|Timeline|SetPlayRate (Variables|Default|GetSmoothSlide) (Variables|Default|GetAnimationSpeed)))