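; BP_LockedDoor is a puzzle door that checks whether its linked unlock mechanisms are done, though it only prints a debug string for now.
; The Construction Script sets UnlockCount to the number of entries in UnlockMechanism.
; Trigger loops over them, raising RealCount for each Done entry and lowering it otherwise, then prints the open message if it equals UnlockCount.
; RealCount is not reset between triggers, so it carries over.
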(event EventTrigger
  (for _array_element (Variables|Default|GetUnlockMechanism)
    (if (Variables|/Game/Code/Puzzles/BP_CombiLock.BP_CombiLock_C|GetDone _array_element)
      (Math|Integer|IncrementInt (Variables|Default|GetRealCount))
      (else
        (Math|Integer|DecrementInt (Variables|Default|GetRealCount)))))
  (if (== (Variables|Default|GetRealCount) (Variables|Default|GetUnlockCount))
    (Development|PrintString "open door")
    (else
      (Development|PrintString "do nothing"))))

(fn ConstructionScript
  (Variables|Default|SetUnlockCount (Utilities|Array|Length (Variables|Default|GetUnlockMechanism))))