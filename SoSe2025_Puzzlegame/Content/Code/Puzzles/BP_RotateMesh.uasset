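; Puzzle actor that swings a pair of door meshes open or to a new yaw when its Trigger event is called.
; A DoOnce limits this to one activation, caching each door's current relative rotation before playing the SmoothRotate timeline from the start.
; The timeline's alpha lerps each door's yaw toward its start value plus a separate left or right rotation offset.
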(event EventBeginPlay)

(event Collision|EventActorBeginOverlap
  (params (OtherActor :type Actor%20Object%20Reference)))

(event EventTick
  (params (DeltaSeconds :type Float%20%28single-precision%29)))

(event EventTrigger
  (params (ActorRef :type Actor%20Object%20Reference) (RemoveActorRef :type Boolean))
  (Utilities|FlowControl|DoOnce false
    (:Completed
      (Variables|Default|SetRelative%20Rotation%20Right (Variables|/Script/Engine.SceneComponent|GetRelativeRotation (Variables|Default|GetDoorRight)))
      (Variables|Default|SetRelative%20Rotation%20Left (Variables|/Script/Engine.SceneComponent|GetRelativeRotation (Variables|Default|GetDoorLeft)))
      (bind _alpha (Timeline|SmoothRotate PlayFromStart)
        (:Update
          (Transformation|SetRelativeRotation (Variables|Default|GetDoorRight) (Math|Rotator|MakeRotator 0.0 0.0 (.yaw (Math|Rotator|Lerp(Rotator) (Math|Rotator|MakeRotator 0.0 0.0 (.yaw (Variables|Default|GetRelative%20Rotation%20Right))) (Math|Rotator|MakeRotator 0.0 0.0 (+ (.yaw (Variables|Default|GetRelative%20Rotation%20Right)) (Variables|Default|GetRotationRight))) _alpha))) false false)
          (Transformation|SetRelativeRotation (Variables|Default|GetDoorLeft) (Math|Rotator|MakeRotator 0.0 0.0 (.yaw (Math|Rotator|Lerp(Rotator) (Math|Rotator|MakeRotator 0.0 0.0 (.yaw (Variables|Default|GetRelative%20Rotation%20Left))) (Math|Rotator|MakeRotator 0.0 0.0 (+ (.yaw (Variables|Default|GetRelative%20Rotation%20Left)) (Variables|Default|GetRotationLeft))) _alpha))) false false))))))

(fn ConstructionScript)