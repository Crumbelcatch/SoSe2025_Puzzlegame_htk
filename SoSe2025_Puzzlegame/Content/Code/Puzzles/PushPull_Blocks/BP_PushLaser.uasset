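; Pushable puzzle block that fires two laser beams to unlock a linked door.
; Player hits snap to an axis, pass a box-trace clearance check, then drive a timeline that slides the block with the player attached.
; While stationary and powered, delayed Tick line traces place both beams and record required BPI_Trigger targets, messaging the door as the count changes.
; Both beams share one last-hit reference, cleared when either trace misses.
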(event Custom|PushBlock
  ;[0.15 0.15 0.15 0.5] Push
  (if (not (Audio|Components|Audio|IsPlaying (Variables|Default|GetMoveBlock)))
    (Variables|Default|SetCurrLocation (Transformation|GetActorLocation))
    (bind _alpha (Timeline|MoveBlock PlayFromStart)
      (:Update
        (Transformation|SetActorRelativeLocation (+ (Variables|Default|GetCurrLocation) (* _alpha (Variables|Default|GetPushDir) (Variables|Default|GetTravelDistance)))))
      (:Finished
        (CallFunction|StopPush)))))

(event Custom|Pew
  (bind _directionalarrow (Variables|Default|GetDirectionalArrow))
  (bind _beamleft (Variables|Default|GetBeamLeft))
  (bind _returnvalue (Transformation|GetWorldLocation _directionalarrow))
  ;[0 0.5828 1 0.5] Pew Left
  (if (Variables|Default|GetIsPowerd)
    (bind _outhit (Collision|LineTraceByChannel _returnvalue (+ _returnvalue (* (Math|Vector|GetForwardVector _directionalarrow) (Variables|Default|GetLaserLength))) "TraceTypeQuery1" false 0 "ForDuration" true "(R=1.000000,G=0.000000,B=0.000000,A=1.000000)" "(R=0.000000,G=1.000000,B=0.000000,A=1.000000)" 2.0))
    (if (.bBlockingHit (Collision|BreakHitResult _outhit))
      (Components|Activation|SetActive _beamleft true false)
      (Niagara|SetNiagaraVariable(Vector3) _beamleft "EndLocation" (.ImpactPoint (Collision|BreakHitResult _outhit)))
      (if (Utilities|DoesObjectImplementInterface (.HitActor (Collision|BreakHitResult _outhit)) "/Game/Code/Interfaces/BPI_Trigger.BPI_Trigger_C")
        (Variables|Default|SetLastHitLeft (.HitActor (Collision|BreakHitResult _outhit)))
        (CallFunction|CheckLocks (.HitActor (Collision|BreakHitResult _outhit))))
      (else
        (Components|Activation|SetActive (Variables|Default|GetBeamLeft) false false)
        (Utilities|Array|RemoveItem (Variables|Default|GetUnlockCount) (Variables|Default|GetLastHitLeft))
        (Variables|Default|SetLastHitLeft 0)
        (Class|BPITrigger|Trigger(Message) (Variables|Default|GetDoorToTrigger) self true)))
    (else
      (Components|Activation|SetActive (Variables|Default|GetBeamLeft) false false))))

(event Custom|StopPush
  (bind _returnvalue (Game|GetPlayerCharacter 0))
  ;[0.15 0.15 0.15 0.5] Stop Push
  (Pawn|Components|CharacterMovement|SetMovementMode (Variables|/Script/Engine.Character|GetCharacterMovement _returnvalue) "MOVE_Walking" 0)
  (Transformation|DetachFromActor _returnvalue "KeepWorld" "KeepWorld" "KeepWorld"))

(event Custom|PewRight
  (bind _directionalarrow1 (Variables|Default|GetDirectionalArrow1))
  (bind _beamright (Variables|Default|GetBeamRight))
  (bind _returnvalue (Transformation|GetWorldLocation _directionalarrow1))
  ;[0 0.5828 1 0.5] Pew Right
  (if (Variables|Default|GetIsPowerd)
    (bind _outhit (Collision|LineTraceByChannel _returnvalue (+ _returnvalue (* (Math|Vector|GetForwardVector _directionalarrow1) (Variables|Default|GetLaserLength))) "TraceTypeQuery1" false 0 "ForDuration" true "(R=1.000000,G=0.000000,B=0.000000,A=1.000000)" "(R=0.000000,G=1.000000,B=0.000000,A=1.000000)" 2.0))
    (if (.bBlockingHit (Collision|BreakHitResult _outhit))
      (Components|Activation|SetActive _beamright true false)
      (Niagara|SetNiagaraVariable(Vector3) _beamright "EndLocation" (.ImpactPoint (Collision|BreakHitResult _outhit)))
      (if (Utilities|DoesObjectImplementInterface (.HitActor (Collision|BreakHitResult _outhit)) "/Game/Code/Interfaces/BPI_Trigger.BPI_Trigger_C")
        (Variables|Default|SetLastHitLeft (.HitActor (Collision|BreakHitResult _outhit)))
        (CallFunction|CheckLocks (.HitActor (Collision|BreakHitResult _outhit))))
      (else
        (Components|Activation|SetActive (Variables|Default|GetBeamRight) false false)
        (Utilities|Array|RemoveItem (Variables|Default|GetUnlockCount) (Variables|Default|GetLastHitLeft))
        (Variables|Default|SetLastHitLeft 0)
        (Class|BPITrigger|Trigger(Message) (Variables|Default|GetDoorToTrigger) self true)))
    (else
      (Components|Activation|SetActive (Variables|Default|GetBeamRight) false false))))

(event Custom|CheckLocks
  (params (InputPin :type Actor%20Object%20Reference%20%28by%20ref%29))
  ;[0.15 0.15 0.15 0.5] CheckLocks
  (if (and (== (Utilities|Array|FindItem (Variables|Default|GetUnlockCount) InputPin) -1) (> (Utilities|Array|FindItem (Variables|Default|GetUnlocksNeeded) InputPin) -1))
    (Utilities|Array|Add (Variables|Default|GetUnlockCount) InputPin)
    (if (== (Utilities|Array|Length (Variables|Default|GetUnlockCount)) (Utilities|Array|Length (Variables|Default|GetUnlocksNeeded)))
      (Class|BPITrigger|Trigger(Message) (Variables|Default|GetDoorToTrigger) self false)
      (else
        (Class|BPITrigger|Trigger(Message) (Variables|Default|GetDoorToTrigger) self true)))))

(event EventTick
  (params (DeltaSeconds :type Float%20%28single-precision%29))
  (if (not (Audio|Components|Audio|IsPlaying (Variables|Default|GetMoveBlock)))
    (Utilities|FlowControl|Delay 0.2)
    (CallFunction|Pew)
    (CallFunction|PewRight)))

(event Collision|EventHit
  (params (MyComp :type Primitive%20Component%20Object%20Reference) (Other :type Actor%20Object%20Reference) (OtherComp :type Primitive%20Component%20Object%20Reference) (bSelfMoved :type Boolean) (HitLocation :type Vector :default "0, 0, 0") (HitNormal :type Vector :default "0, 0, 0") (NormalImpulse :type Vector :default "0, 0, 0") (Hit :type Hit%20Result%20Structure%20%28by%20ref%29))
  (bind _returnvalue (Game|GetPlayerCharacter 0))
  (bind _returnvalue_2 (Transformation|GetActorForwardVector Other))
  (bind (_x _y _z) (Math|Vector|BreakVector _returnvalue_2))
  ;[0.15 0.15 0.15 0.5] Hit Event
  (if (Variables|Default|GetToggleInteract)
    (if (Actor|ActorHasTag Other "Player")
      (Variables|Default|SetPushDir (Math|Vector|MakeVector (Math|Conversions|ToFloat(Integer) (Math|Float|Round _x)) (Math|Conversions|ToFloat(Integer) (Math|Float|Round _y)) (Math|Conversions|ToFloat(Integer) (Math|Float|Round _z))))
      (if (> (Math|Vector|DotProduct HitNormal _returnvalue_2) 0.93)
        (bind _canpush (CallFunction|CanPush))
        (if _canpush
          (Pawn|Components|CharacterMovement|DisableMovement (Variables|/Script/Engine.Character|GetCharacterMovement _returnvalue))
          (Transformation|AttachActorToActor _returnvalue self "None" "KeepWorld" "KeepWorld" "KeepWorld" true)
          (CallFunction|PushBlock))))))

(event EventTrigger
  (params (ActorRef :type Actor%20Object%20Reference) (RemoveActorRef :type Boolean)))

(fn ConstructionScript)

(fn CustomInteractPrompt
  (return ""))

(fn IsInteractable
  (return false))

(fn CanPush
  (bind _returnvalue (Transformation|GetActorLocation))
  (bind _staticmesh (Variables|Default|GetStaticMesh))
  (bind _returnvalue_2 (Class|KismetSystemLibrary|BoxTraceMulti (+ _returnvalue (Math|Vector|MakeVector 5e+01 5e+01 5e+01)) (+ _returnvalue (* (Variables|Default|GetPushDir) (Variables|Default|GetTravelDistance)) (Math|Vector|MakeVector 5e+01 5e+01 5e+01)) (* (Variables|/Script/Engine.SceneComponent|GetRelativeScale3D _staticmesh) (.boxextent (StaticMesh|GetBounds (Variables|/Script/Engine.StaticMeshComponent|GetStaticMesh _staticmesh))) "0.900000,0.900000,0.900000") "0, 0, 0" "TraceTypeQuery1" false 0 "ForDuration" true))
  (return (not _returnvalue_2)))