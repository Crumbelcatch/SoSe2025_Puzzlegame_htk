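; BP_Pushblock is a push/pull block puzzle actor, apparently unfinished.
; BeginPlay finds the tagged BP_Player, caches and logs it, then enables physics on the mesh.
; Tick and Interact do nothing, and IsInteractable returns false.
; Disconnected logic would toggle grabbing, halve or restore player walk speed, and move the block along its forward axis by player input through a swept, interpolated move helper.
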(event EventBeginPlay
  (bind _returnvalue (Actor|GetActorOfClass "/Game/Code/Player/BP_Player.BP_Player_C"))
  (if (Actor|ActorHasTag _returnvalue "Player")
    (bind _output_get (Variables|Default|SetPlayerRef _returnvalue))
    (Development|PrintString (Utilities|String|Append "Player Actor: " (Utilities|GetDisplayName _output_get) "Has been Found by: " (Utilities|GetDisplayName self)))
    (Physics|SetSimulatePhysics (Variables|Components|GetMesh) true)))

(event EventTick
  (params (DeltaSeconds :type Float%20%28single-precision%29))
  (if (Variables|Default|GetToggleInteract)
    _))

(event EventInteract)

(fn ConstructionScript)

(fn IsInteractable
  (return false))