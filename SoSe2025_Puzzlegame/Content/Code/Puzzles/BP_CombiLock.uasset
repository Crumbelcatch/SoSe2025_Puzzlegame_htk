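; BP_CombiLock is an interactable puzzle dial that steps through numbered sides to help unlock a linked Door.
; Each interaction, ignored while rotating, advances the side and turns the mesh pivot with a timeline-driven shortest-path yaw lerp.
; It immediately messages the Door to add or remove itself depending on whether the correct side is selected.
; The construction script computes evenly spaced angles from the side count and warns about out-of-range solutions.
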(event Custom|Rotate
  ;[0 0.6997 0.6456 0.5] Rotate Function
  (bind _alpha (Timeline|SmoothRotate PlayFromStart)
    (:Update
      (Transformation|SetRelativeRotation (Variables|Default|GetMeshPivot) (Math|Rotator|MakeRotator 0.0 0.0 (.yaw (Math|Rotator|Lerp(Rotator) (Math|Rotator|MakeRotator 0.0 0.0 (Variables|Default|GetCurrentRotation)) (Math|Rotator|MakeRotator 0.0 0.0 (Utilities|Array|Get(acopy) (Variables|Default|GetNumbersRotation) (Variables|Default|GetCurrentSide))) _alpha true))) false false))
    (:Finished
      (Variables|Default|SetCurrentRotation (.yaw (Variables|/Script/Engine.SceneComponent|GetRelativeRotation (Variables|Default|GetMeshPivot)))))))

(event EventBeginPlay)

(event EventSetHighlight
  (params (ShowOverlay :type Boolean))
  (Rendering|Material|SetOverlayMaterial (Variables|Default|GetBLOCKOUT_Octagon) (select ShowOverlay "/Game/BLOCKOUT/MapV1_Mat.MapV1_Mat" 0) :!class /Script/Engine.MeshComponent))

(event EventInteract
  ;[0 0.6997 0.6456 0.5] Interact
  (if (not (Audio|Components|Audio|IsPlaying (Variables|Default|GetSmoothRotate)))
    (Math|Integer|IncrementInt (Variables|Default|GetCurrentSide)
      (:%20%20
        (if (== (Variables|Default|GetCurrentSide) (Utilities|Array|Length (Variables|Default|GetNumbersRotation)))
          (Variables|Default|SetCurrentSide 0))
        (CallFunction|Rotate)
        (if (== (Variables|Default|GetCorrectSide) (Variables|Default|GetCurrentSide))
          (Class|BPITrigger|Trigger(Message) (Variables|Default|GetDoor) self false)
          (else
            (Class|BPITrigger|Trigger(Message) (Variables|Default|GetDoor) self true)))))))

(fn ConstructionScript
  (Variables|Default|SetSegmentSize (/ 360 (Variables|Default|GetSides)))
  (for _index (range 0 (Variables|Default|GetSides))
    (if (> 3.6e+02 (* _index (Variables|Default|GetSegmentSize)))
      (Utilities|Array|SetArrayElem (Variables|Default|GetNumbersRotation) _index (* _index (Variables|Default|GetSegmentSize)) true)
      (if (> (Variables|Default|GetCorrectSide) (Variables|Default|GetSides))
        (Development|PrintString (Utilities|String|Append (Utilities|GetDisplayName self) " is unsolvable!  Variable: CorrectSide is bigger than Total Sides") true true "(R=1.000000,G=0.078514,B=0.000000,A=1.000000)" 1e+01)
        (Variables|Default|SetCurrentSide 0)))))

(fn IsInteractable
  (return true))