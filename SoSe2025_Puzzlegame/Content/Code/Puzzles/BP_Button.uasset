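; BP_Button is an interactable puzzle button that only works once it has been powered.
; Receiving a Trigger event powers it permanently, and interacting while powered sends a trigger message to every actor in its ActorsToTrigger list.
; Green and red point lights show the powered state and are refreshed every tick.
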(event EventBeginPlay
  (Rendering|SetVisibility (Variables|Default|GetPointLightGreen) false false)
  (Rendering|SetVisibility (Variables|Default|GetPointLightRed) true false))

(event EventInteract
  (if (Variables|Default|GetIsPowerd)
    (for _array_element (Variables|Default|GetActorsToTrigger)
      (Class|BPITrigger|Trigger(Message) _array_element 0 false))))

(event EventTrigger
  (params (ActorRef :type Actor%20Object%20Reference) (RemoveActorRef :type Boolean))
  (Variables|Default|SetIsPowerd true))

(event EventTick
  (params (DeltaSeconds :type Float%20%28single-precision%29))
  (Rendering|SetVisibility (Variables|Default|GetPointLightGreen) (Variables|Default|GetIsPowerd) false)
  (Rendering|SetVisibility (Variables|Default|GetPointLightRed) (not (Variables|Default|GetIsPowerd)) false))

(fn ConstructionScript)

(fn CustomInteractPrompt
  (return ""))

(fn IsInteractable
  (return true))