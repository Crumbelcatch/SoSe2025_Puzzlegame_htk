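; Component that detects the interactable under the camera's view and drives its highlight.
; Each Tick, a thin Visibility sphere trace runs forward from the camera and checks the hit actor through BPI_Interact.
; A valid new hit becomes CurrentInteractable and is highlighted, while an invalid one clears both.
; Switching directly between interactables un-highlights the new actor before highlighting it, leaving the previous one lit.
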(event EventBeginPlay)

(event EventTick
  (params (DeltaSeconds :type Float%20%28single-precision%29))
  (bind _camera (Variables|Default|GetCamera))
  (bind _returnvalue (Transformation|GetWorldLocation _camera))
  (bind _outhit (Collision|SphereTraceByChannel _returnvalue (+ _returnvalue (* (Math|Vector|GetForwardVector _camera) (Variables|Default|GetForwardMult))) 1.0 "TraceTypeQuery1" false 0 "None" true "(R=1.000000,G=0.000000,B=0.000000,A=1.000000)" "(R=0.000000,G=1.000000,B=0.000000,A=1.000000)" 1.0))
  (bind _isinteractable (Class|BPIInteract|IsInteractable(Message) (.HitActor (Collision|BreakHitResult _outhit))))
  (if (Math|Boolean|ANDBoolean _isinteractable true (Utilities|DoesObjectImplementInterface (.HitActor (Collision|BreakHitResult _outhit)) "/Game/Code/Interfaces/BPI_Interact.BPI_Interact_C"))
    (if (not (== (Variables|Default|GetCurrentInteractable) (.HitActor (Collision|BreakHitResult _outhit))))
      (Class|BPIInteract|SetHighlight(Message) (.HitActor (Collision|BreakHitResult _outhit)) false)
      (bind _output_get (Variables|Default|SetCurrentInteractable (.HitActor (Collision|BreakHitResult _outhit))))
      (Class|BPIInteract|SetHighlight(Message) _output_get true))
    (else
      (Class|BPIInteract|SetHighlight(Message) (Variables|Default|GetCurrentInteractable) false)
      (Variables|Default|SetCurrentInteractable 0))))