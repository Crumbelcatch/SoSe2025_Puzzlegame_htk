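; BP_ToggledDecal is a level utility actor that shows a decal when triggered.
; The construction script applies the DecalMaterial variable to the Decal component.
; BeginPlay hides the whole actor in game and the Trigger event unhides it, with no path that hides it again.
; Leftover Decal SetVisibility nodes are unconnected and never run.
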(event EventTrigger
  (params (ActorRef :type Actor%20Object%20Reference) (RemoveActorRef :type Boolean))
  (Rendering|SetActorHiddenInGame self false))

(event EventBeginPlay
  (Rendering|SetActorHiddenInGame self true))

(fn ConstructionScript
  (Rendering|Components|Decal|SetDecalMaterial (Variables|Default|GetDecal) (Variables|Default|GetDecal%20Material)))