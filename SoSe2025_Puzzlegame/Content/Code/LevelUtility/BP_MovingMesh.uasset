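; BP_MovingMesh is a level utility actor meant to act as a platform moving along the spline of a referenced SplineBP.
; The construction script calls UpdatePosition, which snaps the actor to the world location at DistanceAlongSpline.
; MovePlatform steps that distance by speed and delta time, reversing at the end but never at the start, where MoveForward stays false.
; Tick is empty, and nothing here calls MovePlatform.
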(event Custom|Update%20Position
  (bind _splinebp (Variables|Default|GetSplineBP))
  (bind _spline (Variables|/Game/Code/LevelUtility/BP_TravelSpline.BP_TravelSpline_C|GetSpline _splinebp))
  (Utilities|IsValid _spline
    (:Is%20Valid
      (Transformation|SetActorLocation (Spline|GetLocationatDistanceAlongSpline _spline (Variables|Default|GetDistanceAlongSpline) "World") false false))))

(event Custom|MovePlatform
  (if (Variables|Default|GetMoveForward)
    (if (< (Variables|Default|GetDistanceAlongSpline) (Spline|GetSplineLength (Variables|/Game/Code/LevelUtility/BP_TravelSpline.BP_TravelSpline_C|GetSpline (Variables|Default|GetSplineBP))))
      (Variables|Default|SetDistanceAlongSpline (+ (Variables|Default|GetDistanceAlongSpline) (* (Utilities|Time|GetWorldDeltaSeconds) (Variables|Default|GetMovingSpeed))))
      (else
        (Variables|Default|SetMoveForward false)))
    (elif (> (Variables|Default|GetDistanceAlongSpline) 0.0)
      (Variables|Default|SetDistanceAlongSpline (- (Variables|Default|GetDistanceAlongSpline) (* (Utilities|Time|GetWorldDeltaSeconds) (Variables|Default|GetMovingSpeed))))
      (else
        (Variables|Default|SetMoveForward false)))))

(event EventBeginPlay)

(event Collision|EventActorBeginOverlap
  (params (OtherActor :type Actor%20Object%20Reference)))

(event EventTick
  (params (DeltaSeconds :type Float%20%28single-precision%29)))

(fn ConstructionScript
  (CallFunction|UpdatePosition))