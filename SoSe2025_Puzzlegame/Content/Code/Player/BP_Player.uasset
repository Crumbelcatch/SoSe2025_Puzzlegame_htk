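; Player Blueprint that handles Enhanced Input look and movement and clamps camera pitch on BeginPlay.
; Look input feeds controller yaw and pitch, scaled by LookSensitivity.
; Both move axes apply movement along the same X vector of the control yaw.
; ChangeMappingContext takes a remove flag, but both branches call RemoveMappingContext, including the one labelled as adding.
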(event EventBeginPlay
  (CallFunction|ChangeMappingContext false)
  (CallFunction|SetupCamera))

(event Input|EnhancedActionEvents|EnhancedInputActionIA_Look
  (params (ActionValue :type Vector%202D%20Structure) (ElapsedSeconds :type Float%20%28double-precision%29) (TriggeredSeconds :type Float%20%28double-precision%29) (InputAction :type Input%20Action%20Object%20Reference :default "/Game/Code/Player/Input/IA_Look.IA_Look"))
  ;[0 0.3636 1 0.5] Look
  (Pawn|Input|AddControllerYawInput (* (.x ActionValue) (Variables|Camera|GetLookSensitivity)))
  (bind _result (Math|Float|NegateFloat (.y ActionValue))
    (:%20%20
      (Pawn|Input|AddControllerPitchInput (* _result (Variables|Camera|GetLookSensitivity))))))

(event Input|EnhancedActionEvents|EnhancedInputActionIA_Move
  (params (ActionValue :type Vector%202D%20Structure) (ElapsedSeconds :type Float%20%28double-precision%29) (TriggeredSeconds :type Float%20%28double-precision%29) (InputAction :type Input%20Action%20Object%20Reference :default "/Game/Code/Player/Input/IA_Move.IA_Move"))
  ;[0 0.3636 1 0.5] Move
  (Pawn|Input|AddMovementInput (Math|Rotator|GetRotationXVector (Math|Rotator|MakeRotator 0.0 0.0 (.yaw (Pawn|GetControlRotation :!class /Script/Engine.Pawn)))) (.x ActionValue) false)
  (Pawn|Input|AddMovementInput (Math|Rotator|GetRotationXVector (Math|Rotator|MakeRotator 0.0 0.0 (.yaw (Pawn|GetControlRotation :!class /Script/Engine.Pawn)))) (.y ActionValue) false))

(fn ConstructionScript)

(fn SetupCamera
  (bind _returnvalue (Game|GetPlayerCameraManager 0))
  (Variables|/Script/Engine.PlayerCameraManager|SetViewPitchMin _returnvalue (Variables|Camera|GetCameraPitchMin))
  (Variables|/Script/Engine.PlayerCameraManager|SetViewPitchMax _returnvalue (Variables|Camera|GetCameraPitchMax)))

(fn ChangeMappingContext
  (params (To%20Remove :type Boolean))
  (bind _returnvalue (Game|GetPlayerController 0))
  (bind _returnvalue_2 (Game|GetPlayerController 0))
  (bind _returnvalue_3 (PlayerController|LocalPlayerSubsystems|GetEnhancedInputLocalPlayerSubsystem _returnvalue))
  (bind _returnvalue_4 (PlayerController|LocalPlayerSubsystems|GetEnhancedInputLocalPlayerSubsystem _returnvalue_2))
  (if To%20Remove
    ;[1 0.1198 0.1316 0.5] Remove Mapping Context
    (Utilities|IsValid _returnvalue_4
      (:Is%20Valid
        (Input|RemoveMappingContext _returnvalue_4 0 "(bIgnoreAllPressedKeysUntilRelease=True,bForceImmediately=False,bNotifyUserSettings=False)")))
    (else
      ;[0.2708 1 0.4167 0.5] Add Mapping Context
      (Utilities|IsValid _returnvalue_3
        (:Is%20Valid
          (Input|RemoveMappingContext _returnvalue_3 0 "(bIgnoreAllPressedKeysUntilRelease=True,bForceImmediately=False,bNotifyUserSettings=False)"))))))